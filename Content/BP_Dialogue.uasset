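; BP_Dialogue is a trigger-zone actor that shows dialogue text when the first-person character enters it.
; On overlap it registers itself on the character, creates WBP_Dialogue with its TextToDisplay and swaps Enhanced Input from the default mapping context to the dialogue one.
; SkipDialogue removes the widget and restores default input.
; Leaving the zone only clears the character's reference.
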(event `self.TriggerZone.OnComponentEndOverlap`
  (params (OverlappedComponent :type "PrimitiveComponent Object Reference") (OtherActor :type "Actor Object Reference") (OtherComp :type "PrimitiveComponent Object Reference") (OtherBodyIndex :type Integer))
  (bind _asbp_first_person_character (cast `/Game/FirstPerson/Blueprints/BP_FirstPersonCharacter` OtherActor))
  (set `/Game/FirstPerson/Blueprints/BP_FirstPersonCharacter.BP_Dialogue` null _asbp_first_person_character))

(event `self.TriggerZone.OnComponentBeginOverlap`
  (params (OverlappedComponent :type "PrimitiveComponent Object Reference") (OtherActor :type "Actor Object Reference") (OtherComp :type "PrimitiveComponent Object Reference") (OtherBodyIndex :type Integer) (bFromSweep :type Boolean) (SweepResult :type "HitResult Structure (by ref)"))
  (bind _asbp_first_person_character (cast `/Game/FirstPerson/Blueprints/BP_FirstPersonCharacter` OtherActor))
  (set `/Game/FirstPerson/Blueprints/BP_FirstPersonCharacter.BP_Dialogue` self _asbp_first_person_character)
  (bind _returnvalue (`|CreateWidget` "/Game/WBP_Dialogue.WBP_Dialogue_C"))
  (bind _output_get (set `self.DialogueWidget` _returnvalue))
  (`/Game/WBP_Dialogue.SetDialogueText` _output_get (`self.TextToDisplay`))
  (`UserWidget.AddToViewport` _output_get 0)
  (`self.SwitchPlayerIMC` true))

(event `SwitchPlayerIMC`
  (params (ToDialogue :type Boolean))
  (bind _defaultimc (`self.DefaultIMC`))
  (bind _dialoguesimc (`self.DialoguesIMC`))
  (bind _returnvalue (pcsubsystem `EnhancedInputLocalPlayerSubsystem` (`GameplayStatics.GetPlayerController` 0)))
  (`EnhancedInputSubsystemInterface.RemoveMappingContext` _returnvalue (select `bool` ToDialogue :`false` _dialoguesimc :`true` _defaultimc) (struct))
  (`EnhancedInputSubsystemInterface.AddMappingContext` _returnvalue (select `bool` ToDialogue :`false` _defaultimc :`true` _dialoguesimc) 0 (struct)))

(event `SkipDialogue`
  (`Widget.RemoveFromParent` (`self.DialogueWidget`))
  (`self.SwitchPlayerIMC` false))

(fn `UserConstructionScript`)